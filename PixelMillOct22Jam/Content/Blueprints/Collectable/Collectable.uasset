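; Collectable pickup actor that spins in place and awards score to the flying player.
; Tick accumulates elapsed time and sets absolute roll and pitch from it, scaled by YawFloat, with yaw held at zero.
; When a FlyCharacter overlaps the Collision component, it adds a fixed amount to Score on player 0's FlyController, then destroys itself.
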(event OnComponentBeginOverlap(Collision)
  (params (OverlappedComponent :type Primitive%20Component%20Object%20Reference) (OtherActor :type Actor%20Object%20Reference) (OtherComp :type Primitive%20Component%20Object%20Reference) (OtherBodyIndex :type Integer) (bFromSweep :type Boolean) (SweepResult :type Hit%20Result%20Structure%20%28by%20ref%29))
  (Utilities|Casting|CastToFlyCharacter OtherActor)
  (bind _asfly_controller (Utilities|Casting|CastToFlyController (Game|GetPlayerController 0)))
  (Variables|/Game/Blueprints/PlayerCharacter/FlyController.FlyController_C|SetScore _asfly_controller (+ (Variables|/Game/Blueprints/PlayerCharacter/FlyController.FlyController_C|GetScore _asfly_controller) 10))
  (Actor|DestroyActor))

(event EventTick
  (params (DeltaSeconds :type Float%20%28single-precision%29))
  (Variables|Default|SetTimerFloat (+ DeltaSeconds (Variables|Default|GetTimerFloat)))
  (Transformation|SetActorRotation (Math|Rotator|MakeRotator (* (Variables|Default|GetTimerFloat) (Variables|Default|GetYawFloat)) (* (Variables|Default|GetTimerFloat) (Variables|Default|GetYawFloat)) 0.0)))

(fn ConstructionScript)