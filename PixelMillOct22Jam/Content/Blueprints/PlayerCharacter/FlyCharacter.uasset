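; Player flying character that moves forward every tick and shifts across a 3x3 lane grid via timeline lerps of its Y and Z position.
; Left/right inputs step lanes, down returns to center on release, and upward movement is unwired.
; On BeginPlay, FlyController's carried item count sets max fly speed (more is slower) and visible item components.
; DealDamage reduces controller health; a separate AnyDamage/M-key test uses local Health, both only printing results.
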(event Custom|GameOver
  (Development|PrintString "you are unalive"))

(event Custom|ChangeLaneY
  (params (Shift%20Lane :type Integer))
  (bind _returnvalue (Transformation|GetActorLocation))
  (bind (_x _y) (Math|Vector|BreakVector _returnvalue))
  ;[1 1 1 1 25] Y-Axis Movement
  (Variables|Y-Axis|SetTargetLaneIndexY (Math|Integer|Clamp(Integer) (+ Shift%20Lane (Variables|Y-Axis|GetCurrentLaneIndexY)) 0 2))
  (Variables|Y-Axis|SetCurrentZPosition (.Z (Math|Vector|BreakVector (Transformation|GetActorLocation))))
  (bind _verp_speed (Timeline|Timeline_0 PlayFromStart)
    (:Update
      (Transformation|SetActorLocation (Math|Vector|MakeVector _x _y (Math|Float|Lerp (Variables|Y-Axis|GetCurrentZPosition) (Utilities|Array|Get(acopy) (Variables|Y-Axis|GetLanePositionY) (Variables|Y-Axis|GetTargetLaneIndexY)) _verp_speed)) false false)
      (Variables|Y-Axis|SetCurrentLaneIndexY (Variables|Y-Axis|GetTargetLaneIndexY)))))

(event Custom|ChangeLaneX
  (params (Shift%20Lane :type Integer))
  (bind _returnvalue (Transformation|GetActorLocation))
  (bind (_x _y _z) (Math|Vector|BreakVector _returnvalue))
  ;[1 1 1 1 25] X-Axis Movement
  (Variables|X-Axis|SetTargetLaneIndexX (Math|Integer|Clamp(Integer) (+ Shift%20Lane (Variables|X-Axis|GetCurrentLaneIndexX)) 0 2))
  (Variables|X-Axis|SetCurrentYPosition (.Y (Math|Vector|BreakVector (Transformation|GetActorLocation))))
  (bind _verp_speed (Timeline|ChangeLaneTransition PlayFromStart)
    (:Update
      (Transformation|SetActorLocation (Math|Vector|MakeVector _x (Math|Float|Lerp (Variables|X-Axis|GetCurrentYPosition) (Utilities|Array|Get(acopy) (Variables|X-Axis|GetLanePositionX) (Variables|X-Axis|GetTargetLaneIndexX)) _verp_speed) _z) false false)
      (Variables|X-Axis|SetCurrentLaneIndexX (Variables|X-Axis|GetTargetLaneIndexX)))))

(event Custom|ReturnToOriginX
  (bind _returnvalue (Transformation|GetActorLocation))
  (bind (_x _y _z) (Math|Vector|BreakVector _returnvalue))
  ;[1 1 1 1 25] X-Axis Movement
  (if (!= (Variables|X-Axis|GetCurrentLaneIndexX) 1)
    (Variables|X-Axis|SetTargetLaneIndexX 1)
    (Variables|X-Axis|SetCurrentYPosition (.Y (Math|Vector|BreakVector (Transformation|GetActorLocation))))
    (bind _verp_speed (Timeline|RevertLaneTransition PlayFromStart)
      (:Update
        (Transformation|SetActorLocation (Math|Vector|MakeVector _x (Math|Float|Lerp (Variables|X-Axis|GetCurrentYPosition) (Utilities|Array|Get(acopy) (Variables|X-Axis|GetLanePositionX) 1) _verp_speed) _z) false false))
      (:Finished
        (Variables|X-Axis|SetCurrentLaneIndexX (Variables|X-Axis|GetTargetLaneIndexX))))))

(event Custom|ReturnToOriginY
  (bind _returnvalue (Transformation|GetActorLocation))
  (bind (_x _y) (Math|Vector|BreakVector _returnvalue))
  ;[1 1 1 1 25] Y-Axis Movement
  (if (!= (Variables|Y-Axis|GetCurrentLaneIndexY) 1)
    (Variables|Y-Axis|SetTargetLaneIndexY 1)
    (Variables|Y-Axis|SetCurrentZPosition (.Z (Math|Vector|BreakVector (Transformation|GetActorLocation))))
    (bind _verp_speed (Timeline|Timeline_1 PlayFromStart)
      (:Update
        (Transformation|SetActorLocation (Math|Vector|MakeVector _x _y (Math|Float|Lerp (Variables|Y-Axis|GetCurrentZPosition) (Utilities|Array|Get(acopy) (Variables|Y-Axis|GetLanePositionY) 1) _verp_speed)) false false))
      (:Finished
        (Variables|Y-Axis|SetCurrentLaneIndexY (Variables|Y-Axis|GetTargetLaneIndexY))))))

(event Game|Damage|EventAnyDamage
  (params (Damage :type Float%20%28single-precision%29) (DamageType :type Damage%20Type%20Object%20Reference) (InstigatedBy :type Controller%20Object%20Reference) (DamageCauser :type Actor%20Object%20Reference))
  ;[1 1 1] Testing Health
  (Variables|HealthComponents|SetHealth (- (Variables|HealthComponents|GetHealth) Damage))
  (if (<= (Variables|HealthComponents|GetHealth) 0.0)
    (Development|PrintString "Dead")
    (else
      (Development|PrintString (Utilities|String|ToString(Float) (Variables|HealthComponents|GetHealth))))))

(event EventDealDamage
  (params (DamageOutput :type Integer))
  ;[1 1 1 1 20] Receiving End of Deal Damage to Player
  (bind _asfly_controller (Utilities|Casting|CastToFlyController (Game|GetPlayerController 0)))
  (bind _output_get (Variables|/Game/Blueprints/PlayerCharacter/FlyController.FlyController_C|SetHealth _asfly_controller (- (Variables|/Game/Blueprints/PlayerCharacter/FlyController.FlyController_C|GetHealth _asfly_controller) DamageOutput)))
  (if (== _output_get 0)
    (CallFunction|GameOver)
    (else
      (Development|PrintString "damage dealt"))))

(event EventTick
  (params (DeltaSeconds :type Float%20%28single-precision%29))
  ;[1 1 1] Per tick player moves (x) amount of units
  (Pawn|Input|AddMovementInput (Math|Vector|GetForwardVector (Math|Rotator|MakeRotator (.Yaw (Math|Rotator|BreakRotator (Pawn|GetControlRotation :!class /Script/Engine.Pawn))) 0.0 0.0)) 1.0 false))

(event EventBeginPlay
  (bind _charactermovement (Variables|Character|GetCharacterMovement))
  (bind _asfly_controller (Utilities|Casting|CastToFlyController (Game|GetPlayerController 0)))
  (switch int (Variables|/Game/Blueprints/PlayerCharacter/FlyController.FlyController_C|GetCurrentItemCarry _asfly_controller)
    (:0
      (Variables|/Script/Engine.CharacterMovementComponent|SetMaxFlySpeed _charactermovement 2.5e+03)
      (Rendering|SetVisibility (Variables|Default|GetTempItem_1) false false)
      (Rendering|SetVisibility (Variables|Default|GetTempItem_2) false false)
      (Rendering|SetVisibility (Variables|Default|GetTempItem_3) false false)
      (Rendering|SetVisibility (Variables|Default|GetTempItem_4) false false)
      (Rendering|SetVisibility (Variables|Default|GetTempItem_5) false false))
    (:1
      (Variables|/Script/Engine.CharacterMovementComponent|SetMaxFlySpeed _charactermovement 2.2e+03)
      (Rendering|SetVisibility (Variables|Default|GetTempItem_1) true false)
      (Rendering|SetVisibility (Variables|Default|GetTempItem_2) false false)
      (Rendering|SetVisibility (Variables|Default|GetTempItem_3) false false)
      (Rendering|SetVisibility (Variables|Default|GetTempItem_4) false false)
      (Rendering|SetVisibility (Variables|Default|GetTempItem_5) false false))
    (:2
      (Variables|/Script/Engine.CharacterMovementComponent|SetMaxFlySpeed _charactermovement 1.9e+03)
      (Rendering|SetVisibility (Variables|Default|GetTempItem_1) true false)
      (Rendering|SetVisibility (Variables|Default|GetTempItem_2) true false)
      (Rendering|SetVisibility (Variables|Default|GetTempItem_3) false false)
      (Rendering|SetVisibility (Variables|Default|GetTempItem_4) false false)
      (Rendering|SetVisibility (Variables|Default|GetTempItem_5) false false))
    (:3
      (Variables|/Script/Engine.CharacterMovementComponent|SetMaxFlySpeed _charactermovement 1.6e+03)
      (Rendering|SetVisibility (Variables|Default|GetTempItem_1) true false)
      (Rendering|SetVisibility (Variables|Default|GetTempItem_2) true false)
      (Rendering|SetVisibility (Variables|Default|GetTempItem_3) true false)
      (Rendering|SetVisibility (Variables|Default|GetTempItem_4) false false)
      (Rendering|SetVisibility (Variables|Default|GetTempItem_5) false false))
    (:4
      (Variables|/Script/Engine.CharacterMovementComponent|SetMaxFlySpeed _charactermovement 1.3e+03)
      (Rendering|SetVisibility (Variables|Default|GetTempItem_1) true false)
      (Rendering|SetVisibility (Variables|Default|GetTempItem_2) true false)
      (Rendering|SetVisibility (Variables|Default|GetTempItem_3) true false)
      (Rendering|SetVisibility (Variables|Default|GetTempItem_4) true false)
      (Rendering|SetVisibility (Variables|Default|GetTempItem_5) false false))
    (:5
      (Variables|/Script/Engine.CharacterMovementComponent|SetMaxFlySpeed _charactermovement 1e+03)
      (Rendering|SetVisibility (Variables|Default|GetTempItem_1) true false)
      (Rendering|SetVisibility (Variables|Default|GetTempItem_2) true false)
      (Rendering|SetVisibility (Variables|Default|GetTempItem_3) true false)
      (Rendering|SetVisibility (Variables|Default|GetTempItem_4) true false)
      (Rendering|SetVisibility (Variables|Default|GetTempItem_5) true false))))

(event Input|ActionEvents|InputActionMoveLeft
  (params (Key :type Key%20Structure :default "None"))
  ;[1 1 1] Move Left/Right
  (:Pressed
    (CallFunction|ChangeLaneX -1)))

(event Input|ActionEvents|InputActionMoveRight
  (params (Key :type Key%20Structure :default "None"))
  ;[1 1 1] Move Left/Right
  (:Pressed
    (CallFunction|ChangeLaneX 1)))

(event Input|ActionEvents|InputActionMoveUp
  (params (Key :type Key%20Structure :default "None"))
  ;[1 1 1] Move Up/Down
)

(event Input|ActionEvents|InputActionMoveDown
  (params (Key :type Key%20Structure :default "None"))
  ;[1 1 1] Move Up/Down
  (:Pressed
    (CallFunction|ChangeLaneY -1))
  (:Released
    (CallFunction|ReturntoOriginY)))

(event Input|KeyboardEvents|M
  (params (Key :type Key%20Structure :default "None"))
  ;[1 1 1] Testing Health
  (:Pressed
    (Game|Damage|ApplyDamage self 1.0 0 0)))

(fn ConstructionScript)