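; FlyCharacter_1 is a player character Blueprint that moves forward automatically and switches between three lanes, in the style of a lane runner.
; Tick forces forward movement input, using a rotator with control yaw wired into roll, so the direction stays world X.
; MoveLeft and MoveRight call ChangeLane, which clamps the target index and uses a timeline to lerp actor Y to that lane's position.
; The current lane index updates only when the timeline finishes.
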(event Custom|ChangeLane
  (params (Shift%20Lane :type Integer))
  (bind _returnvalue (Transformation|GetActorLocation))
  (bind (_x _y _z) (Math|Vector|BreakVector _returnvalue))
  (Variables|Default|SetTargetLaneIndex (Math|Integer|Clamp(Integer) (+ Shift%20Lane (Variables|Default|GetCurrentLaneIndex)) 0 2))
  (Variables|Default|SetCurrentYPosition (.Y (Math|Vector|BreakVector (Transformation|GetActorLocation))))
  (bind _verp_speed (Timeline|ChangeLaneTransition PlayFromStart)
    (:Update
      (Transformation|SetActorLocation (Math|Vector|MakeVector _x (Math|Float|Lerp (Variables|Default|GetCurrentYPosition) (Utilities|Array|Get(acopy) (Variables|Default|GetLanePosition) (Variables|Default|GetTargetLaneIndex)) _verp_speed) _z) false false))
    (:Finished
      (Variables|Default|SetCurrentLaneIndex (Variables|Default|GetTargetLaneIndex)))))

(event EventTick
  (params (DeltaSeconds :type Float%20%28single-precision%29))
  ;[1 1 1] Per tick player moves (x) amount of units
  (Pawn|Input|AddMovementInput (Math|Vector|GetForwardVector (Math|Rotator|MakeRotator (.Yaw (Math|Rotator|BreakRotator (Pawn|GetControlRotation :!class /Script/Engine.Pawn))) 0.0 0.0)) 1.0 true))

(event Input|ActionEvents|InputActionMoveLeft
  (params (Key :type Key%20Structure :default "None"))
  (:Pressed
    (CallFunction|ChangeLane -1)))

(event Input|ActionEvents|InputActionMoveRight
  (params (Key :type Key%20Structure :default "None"))
  (:Pressed
    (CallFunction|ChangeLane 1)))

(fn ConstructionScript)